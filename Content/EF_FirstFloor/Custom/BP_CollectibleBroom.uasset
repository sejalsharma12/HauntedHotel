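; BP_CollectibleBroom is a broom pickup that the player collects with Enter.
; Its Sphere overlap enables input for FirstPersonCharacter and disables it on exit.
; Collecting decrements CollectiblesLeft on FirstPersonGameMode, destroys the actor and, at zero, shows the L1KeyInst widget.
; The widget's timed removal follows DestroyActor, so that Delay likely never completes.
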(event OnComponentBeginOverlap(Sphere)
  (params (OverlappedComponent :type Primitive%20Component%20Object%20Reference) (OtherActor :type Actor%20Object%20Reference) (OtherComp :type Primitive%20Component%20Object%20Reference) (OtherBodyIndex :type Integer) (bFromSweep :type Boolean) (SweepResult :type Hit%20Result%20Structure%20%28by%20ref%29))
  (Utilities|Casting|CastToFirstPersonCharacter OtherActor)
  (Input|EnableInput (Game|GetPlayerController 0)))

(event OnComponentEndOverlap(Sphere)
  (params (OverlappedComponent :type Primitive%20Component%20Object%20Reference) (OtherActor :type Actor%20Object%20Reference) (OtherComp :type Primitive%20Component%20Object%20Reference) (OtherBodyIndex :type Integer))
  (Utilities|Casting|CastToFirstPersonCharacter OtherActor)
  (Input|DisableInput 0))

(event EventBeginPlay)

(event Collision|EventActorBeginOverlap
  (params (OtherActor :type Actor%20Object%20Reference)))

(event EventTick
  (params (DeltaSeconds :type Float%20%28single-precision%29)))

(event Input|KeyboardEvents|Enter
  (params (Key :type Key%20Structure :default "None"))
  (:Pressed
    (bind _asfirst_person_game_mode (Utilities|Casting|CastToFirstPersonGameMode (Game|GetGameMode)))
    (bind _result (Math|Integer|DecrementInt (Variables|/Game/FirstPersonBP/Blueprints/FirstPersonGameMode.FirstPersonGameMode_C|GetCollectiblesLeft _asfirst_person_game_mode))
      (:%20%20
        (bind _output_get (Variables|/Game/FirstPersonBP/Blueprints/FirstPersonGameMode.FirstPersonGameMode_C|SetCollectiblesLeft _asfirst_person_game_mode _result))
        (Actor|DestroyActor)
        (if (== _output_get 0)
          (bind _returnvalue (UserInterface|CreateWidget "/Game/UI/L1KeyInst.L1KeyInst_C"))
          (UserInterface|Viewport|AddtoViewport _returnvalue 0)
          (Utilities|FlowControl|Delay 2e+01)
          (Widget|RemovefromParent _returnvalue))))))

(fn ConstructionScript)